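; DeskStandCopy is an actor that serves as an alternate camera view the player can toggle with the interaction key, apparently for standing at a desk.
; r_Function takes a Condition and binds to the BeginInteraction dispatcher on BP_FirstPersonCharacter.
; While Condition is true, each press flip-flops a blended view target between this actor and the player character.
; The older wall-lean chain, including its movement and input handling, is disabled.
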(event `self.Receiver_Function`
  (params (Condition :type Boolean))
  (bind _asbp_first_person_character (cast `/Game/FirstPerson/Blueprints/BP_FirstPersonCharacter` (`GameplayStatics.GetPlayerCharacter` 0)))
  (add `/Game/FirstPerson/Blueprints/BP_FirstPersonCharacter.Begin Interaction` _asbp_first_person_character (delegate `Begin Interaction Key Pressed`)))

(event `Begin Interaction Key Pressed`
  (bind _returnvalue (`GameplayStatics.GetPlayerController` 0))
  (if (stale `self.Receiver_Function` Condition)
    (`/Engine/EditorBlueprintResources/StandardMacros.FlipFlop`
      (:`A`
        (`PlayerController.SetViewTargetWithBlend` _returnvalue self 0.5 "VTBlend_Linear" 0.0 false))
      (:`B`
        (`PlayerController.SetViewTargetWithBlend` _returnvalue (`GameplayStatics.GetPlayerCharacter` 0) 0.5 "VTBlend_Linear" 0.0 false)))
    (`KismetSystemLibrary.Delay` 0.5 :!enabledstate Disabled)
    (`self.EnableInput` null :!enabledstate Disabled)))

(fn `UserConstructionScript`)